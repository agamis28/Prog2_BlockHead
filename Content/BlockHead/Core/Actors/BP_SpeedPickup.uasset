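; BP_SpeedPickup is a pickup actor that gives the player a temporary speed boost on overlap.
; It raises the player's ForwardForce, shows a WBP_SpeedBoost widget and hides its PickupFX while the effect runs.
; After SpeedDuration it removes the widget and briefly applies a strong negative force to brake, then restores a hardcoded normal force and destroys itself.
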(event `self.ReceiveActorBeginOverlap`
  (params (OtherActor :type "Actor Object Reference"))
  ;[0.1062 1 0.2026] When Colliding With Player Increase Forward Force
  (bind _asbp_player (cast `/Game/BlockHead/Core/Actors/BP_Player` OtherActor))
  (set `self.Player` _asbp_player)
  (set `/Game/BlockHead/Core/Actors/BP_Player.ForwardForce` 6000.0 (`self.Player`))
  ;[0.1062 1 0.2026] Creating Speed Boost Widget UII
  (bind _returnvalue (`|CreateWidget` "/Game/BlockHead/Core/UI/WBP_SpeedBoost.WBP_SpeedBoost_C" (`GameplayStatics.GetPlayerController` 0)))
  (bind _output_get (set `self.SpeedBoostUI` _returnvalue))
  (`UserWidget.AddToViewport` _output_get 0)
  ;[0.1062 1 0.2026] Make Pickup Invisible Then Slow Down Force After Delay and Remove Widget, Then Return to Normal Forward Force And Destroy
  (`SceneComponent.SetVisibility` (`self.PickupFX`) false false)
  (`KismetSystemLibrary.Delay` (`self.SpeedDuration`))
  (set `/Game/BlockHead/Core/Actors/BP_Player.ForwardForce` -20000.0 (`self.Player`))
  (`Widget.RemoveFromParent` (`self.SpeedBoostUI`))
  (`KismetSystemLibrary.Delay` 0.5)
  (set `/Game/BlockHead/Core/Actors/BP_Player.ForwardForce` 1000.0 (`self.Player`))
  (`self.K2_DestroyActor`))

(fn `UserConstructionScript`)