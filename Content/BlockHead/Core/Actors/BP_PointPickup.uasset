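; BP_PointPickup is a score pickup actor that adds its value to the game's total score when collected.
; On BeginPlay it casts and caches the BP_GameInstance reference.
; Any actor overlap, with no check for the player, adds PickupValue to the TotalScore held on the game instance, then destroys the pickup.
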(event `self.ReceiveBeginPlay`
  ;[0.1062 1 0.2026] Setting Reference to Game Instance
  (bind _asbp_game_instance (cast `/Game/BlockHead/Core/Game/BP_GameInstance` (`GameplayStatics.GetGameInstance`)))
  (set `self.GameInstance` _asbp_game_instance))

(event `self.ReceiveActorBeginOverlap`
  (params (OtherActor :type "Actor Object Reference"))
  ;[0.1062 1 0.2026] When Player Touches Pickup Increment Game Instance Total Score by Pickup Value, Then Destroy Pickup
  (set `/Game/BlockHead/Core/Game/BP_GameInstance.TotalScore` (+ (`/Game/BlockHead/Core/Game/BP_GameInstance.TotalScore` (`self.GameInstance`)) (`self.PickupValue`)) (`self.GameInstance`))
  (`self.K2_DestroyActor`))

(fn `UserConstructionScript`)